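; TestEnemy is an unfinished melee enemy AI Blueprint whose See Pawn event is empty, leaving its chase-and-attack logic disconnected.
; That unused chain moves to the player, then plays an axe attack montage and whoosh sound, gated by a CanAttack flag that resets when the montage completes or is interrupted.
; The montage notify would call AttackDamage and KnockBack, both empty functions.
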(event OnSeePawn(PawnSensing)
  (params (Pawn :type Pawn%20Object%20Reference))
  ;[0.15 0.15 0.15 0.5] Enemy AI
)

(event EventBeginPlay)

(event Collision|EventActorBeginOverlap
  (params (OtherActor :type Actor%20Object%20Reference)))

(event EventTick
  (params (DeltaSeconds :type Float%20%28single-precision%29)))

(fn ConstructionScript)

(fn AttackDamage)

(fn KnockBack)