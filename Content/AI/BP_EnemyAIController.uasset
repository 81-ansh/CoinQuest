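; Enemy AI controller that runs the BT_Enemy behavior tree and feeds its blackboard with target information.
; AI perception updates set TargetActor when a BP_ThirdPersonCharacter is sensed and clear it when that character is lost.
; Each tick, it sets IsInRange from whether the controlled pawn is within a short fixed distance of the target.
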(event OnTargetPerceptionUpdated(AIPerception)
  (params (Actor :type Actor%20Object%20Reference) (Stimulus :type AI%20Stimulus%20Structure))
  (Utilities|Casting|CastToBP_ThirdPersonCharacter Actor)
  (if (.bSuccessfullySensed (Utilities|Struct|BreakAIStimulus Stimulus))
    (AI|Components|Blackboard|SetValueasObject (AI|GetBlackboard 0) (Utilities|Name|MakeLiteralName "TargetActor") Actor)
    (else
      (AI|Components|Blackboard|SetValueasObject (AI|GetBlackboard 0) (Utilities|Name|MakeLiteralName "TargetActor") 0))))

(event EventBeginPlay
  (AI|RunBehaviorTree "/Game/AI/BT_Enemy.BT_Enemy"))

(event EventTick
  (params (DeltaSeconds :type Float%20%28single-precision%29))
  (bind _returnvalue (AI|GetBlackboard 0))
  (bind _returnvalue_2 (Utilities|Name|MakeLiteralName "TargetActor"))
  (bind _returnvalue_3 (AI|Components|Blackboard|GetValueasObject _returnvalue _returnvalue_2))
  (bind _asactor (Utilities|Casting|CastToActor _returnvalue_3))
  (Utilities|IsValid _returnvalue_3
    (:Is%20Valid
      (AI|Components|Blackboard|SetValueasBool _returnvalue (Utilities|Name|MakeLiteralName "IsInRange") (< (Transformation|GetDistanceTo _asactor (Pawn|GetControlledPawn)) 2e+02)))))

(fn ConstructionScript)